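; BP_Crossplay is a Blueprint that reports the player's position to a local HTTP server for a crossplay bridge.
; On BeginPlay it sends an empty JSON POST to a connect endpoint through the VaRest plugin.
; Every Tick it builds a new VaRest POST carrying player 0's character X, Y and Z location to a player endpoint, without handling responses.
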(event EventBeginPlay
  (bind _returnvalue (Class|VaRestSubsystem|ConstructVaRestRequestExt (|VaRestSubsystem) "POST" "json"))
  (Class|VaRestRequestJSON|SetURL _returnvalue "http://127.0.0.1:25570/ue4/connect")
  (Class|VaRestRequestJSON|ExecuteProcessRequest _returnvalue))

(event Collision|EventActorBeginOverlap
  (params (OtherActor :type Actor%20Object%20Reference)))

(event EventTick
  (params (DeltaSeconds :type Float%20%28single-precision%29))
  (bind _returnvalue (Game|GetPlayerCharacter 0))
  (bind _returnvalue_2 (Transformation|GetActorLocation _returnvalue))
  (bind (_x _y _z) (Math|Vector|BreakVector _returnvalue_2))
  (bind _returnvalue_3 (Class|VaRestSubsystem|ConstructVaRestRequestExt (|VaRestSubsystem) "POST" "json"))
  (Class|VaRestJsonObject|SetNumberField (Class|VaRestRequestJSON|GetRequestObject _returnvalue_3) "x" _x)
  (Class|VaRestJsonObject|SetNumberField (Class|VaRestRequestJSON|GetRequestObject _returnvalue_3) "y" _y)
  (Class|VaRestJsonObject|SetNumberField (Class|VaRestRequestJSON|GetRequestObject _returnvalue_3) "z" _z)
  (Class|VaRestRequestJSON|SetURL _returnvalue_3 "http://127.0.0.1:25570/player")
  (Class|VaRestRequestJSON|ExecuteProcessRequest _returnvalue_3))

(fn ConstructionScript)